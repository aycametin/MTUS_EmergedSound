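; Player controller for the SoundWall grid game, where the user places coloured panels on a wall.
; Forwards movement, zoom and right-drag look input to BP_CameraController, while keys pick user colour and start play or music through WallGridManager.
; A preview actor follows a cursor trace snapped to the grid.
; Left click on valid placement marks the cell and its neighbours with the user type, after sampling track amplitude whose threshold branch is empty.
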(event `self.ReceiveBeginPlay`
  (`self.SetPlacementModeEnabled` true))

(event `InputAxis|CameraOrbit`
  (params (AxisValue :type "Float (single-precision)"))
  (bind _asbp_camera_controller (cast `/Game/SoundWall/BP_CameraController` (`self.K2_GetPawn`)))
  (`/Game/SoundWall/BP_CameraController.CameraOrbit` _asbp_camera_controller AxisValue))

(event `InputAxis|MoveForward/Backward`
  (params (AxisValue :type "Float (single-precision)"))
  (bind _asbp_camera_controller (cast `/Game/SoundWall/BP_CameraController` (`self.K2_GetPawn`)))
  (`/Game/SoundWall/BP_CameraController.MoveForward` _asbp_camera_controller AxisValue))

(event `InputAxis|SrafeLeft/Right`
  (params (AxisValue :type "Float (single-precision)"))
  (bind _asbp_camera_controller (cast `/Game/SoundWall/BP_CameraController` (`self.K2_GetPawn`)))
  (`/Game/SoundWall/BP_CameraController.LeftRightStrafe` _asbp_camera_controller AxisValue))

(event `InputAction|CameraZoomIn`
  (params (Key :type "Key Structure"))
  (:`Pressed`
    (bind _asbp_camera_controller (cast `/Game/SoundWall/BP_CameraController` (`self.K2_GetPawn`)))
    (`/Game/SoundWall/BP_CameraController.CameraZoom` _asbp_camera_controller -1.0)))

(event `InputAction|CameraZoomOut`
  (params (Key :type "Key Structure"))
  (:`Pressed`
    (bind _asbp_camera_controller (cast `/Game/SoundWall/BP_CameraController` (`self.K2_GetPawn`)))
    (`/Game/SoundWall/BP_CameraController.CameraZoom` _asbp_camera_controller 1.0)))

(event `InputAxis|CameraPitch`
  (params (AxisValue :type "Float (single-precision)"))
  (bind _asbp_camera_controller (cast `/Game/SoundWall/BP_CameraController` (`self.K2_GetPawn`)))
  (`/Game/SoundWall/BP_CameraController.CameraPitch` _asbp_camera_controller AxisValue))

(event `InputAction|MouseRightClick`
  (params (Key :type "Key Structure"))
  (:`Pressed`
    (set `self.RightButtonPressed` true))
  (:`Released`
    (set `self.RightButtonPressed` false)))

(event `InputAxis|MouseX`
  (params (AxisValue :type "Float (single-precision)"))
  (if (`self.RightButtonPressed`)
    (bind _asbp_camera_controller (cast `/Game/SoundWall/BP_CameraController` (`self.K2_GetPawn`)))
    (`/Game/SoundWall/BP_CameraController.CameraOrbit` _asbp_camera_controller AxisValue)))

(event `InputAxis|MouseY`
  (params (AxisValue :type "Float (single-precision)"))
  (if (`self.RightButtonPressed`)
    (bind _asbp_camera_controller (cast `/Game/SoundWall/BP_CameraController` (`self.K2_GetPawn`)))
    (`/Game/SoundWall/BP_CameraController.CameraPitch` _asbp_camera_controller AxisValue)))

(event `self.ReceiveTick`
  (params (DeltaSeconds :type "Float (single-precision)"))
  (if (`self.PlacementModeEnabled`)
    (`self.UpdatePlacement`)))

(event `InputAction|MouseLeftClick`
  (params (Key :type "Key Structure"))
  (:`Pressed`
    (if (`self.PlacementModeEnabled`)
      (`self.SpawnPanel`))))

(event `Key|F6`
  (params (Key :type "Key Structure"))
  ;[1 1 1] Start Play Button
  (:`Pressed`
    (bind _returnvalue (`GameplayStatics.GetActorOfClass` "/Game/SoundWall/SoundWallGrid/WallGridManager.WallGridManager_C"))
    (set `/Game/SoundWall/SoundWallGrid/WallGridManager.Start` true _returnvalue)))

(event `Key|Four`
  (params (Key :type "Key Structure"))
  ;[1 1 1] Start Music Button
  (:`Pressed`
    (bind _returnvalue (`GameplayStatics.GetActorOfClass` "/Game/SoundWall/SoundWallGrid/WallGridManager.WallGridManager_C"))
    (`/Game/SoundWall/SoundWallGrid/WallGridManager.StartMusicEvent` _returnvalue)))

(event `Key|One`
  (params (Key :type "Key Structure"))
  ;[1 1 1] User Color Assignment
  (:`Pressed`
    (set `self.User` "NewEnumerator1")))

(event `Key|Two`
  (params (Key :type "Key Structure"))
  ;[1 1 1] User Color Assignment
  (:`Pressed`
    (set `self.User` "NewEnumerator5")))

(event `Key|Three`
  (params (Key :type "Key Structure"))
  ;[1 1 1] User Color Assignment
  (:`Pressed`
    (set `self.User` "NewEnumerator6")))

(fn `SetPlacementModeEnabled`
  (params (IsEnabled :type Boolean))
  (bind _placeableactor (`self.PlaceableActor`))
  (if (== IsEnabled (`self.PlacementModeEnabled`))
    (return)
    (else
      (bind _output_get (set `self.PlacementModeEnabled` IsEnabled))
      (if _output_get
        (bind _returnvalue (`|SpawnActorFromClass` (`self.PlaceableActorType`) (`KismetMathLibrary.MakeTransform` (0.0 0.0 0.0)) "AlwaysSpawn" "OverrideRootScale" null null))
        (bind _output_get_2 (set `self.PlaceableActor` _returnvalue))
        (bind _returnvalue_2 (`self.GetComponentByClass` _output_get_2 "/Game/SoundWall/WallObjects/BP_ClickableComponents.BP_ClickableComponents_C"))
        (`/Engine/EditorBlueprintResources/StandardMacros.IsValid` _returnvalue_2
          (:`Is Valid`
            (`/Game/SoundWall/WallObjects/BP_ClickableComponents.InPlacementMode` _returnvalue_2))
          (:`Is Not Valid`
            _))
        (`AddComponent|NODE_AddBP_PloppableComponent-0` :`self` _output_get_2)
        (else
          (`/Engine/EditorBlueprintResources/StandardMacros.IsValid` _placeableactor
            (:`Is Valid`
              (`self.K2_DestroyActor` _placeableactor))))))))

(fn `SpawnPanel`
  (bind _returnvalue (`self.GetComponentByClass` (`self.PlaceableActor`) "/Game/SoundWall/WallObjects/BP_PloppableComponent.BP_PloppableComponent_C"))
  (`/Engine/EditorBlueprintResources/StandardMacros.IsValid` _returnvalue
    (:`Is Valid`
      (if (`/Game/SoundWall/WallObjects/BP_PloppableComponent.IsPlacementValid` _returnvalue)
        (bind _returnvalue_2 (`GameplayStatics.GetActorOfClass` "/Game/SoundWall/SoundWallGrid/WallGridManager.WallGridManager_C"))
        (bind _outputvector (`/Game/SoundWall/SoundWallGrid/WallGridManager.GetClosestGridCell` _returnvalue_2 (`self.K2_GetActorLocation` (`self.PlaceableActor`))))
        ;[1 1 1] Amplitude Value
        (bind _outamplitudes (`SoundVisualizationStatics.GetAmplitude` (`self.Track`) 0 (`KismetMathLibrary.Abs` (+ (`KismetSystemLibrary.GetGameTimeInSeconds`) 2.0)) 0.1 10))
        (if (`KismetArrayLibrary.Array_IsValidIndex` _outamplitudes 9)
          (if (>= (* (`KismetMathLibrary.Abs` (`|GetArrayItem` _outamplitudes 9)) 0.001) 5.0)
            _
            (else
              _))
          (`/Game/SoundWall/SoundWallGrid/GridCells.SetOccupied` _outputvector (`self.User`) null)
          (`/Game/SoundWall/SoundWallGrid/GridCells.Set All Neighbours` _outputvector (`self.User`)))))))

(fn `UpdatePlacement`
  (bind (_worldlocation _worlddirection) (`self.DeprojectMousePositionToWorld`))
  (bind _outhit (`KismetSystemLibrary.LineTraceSingle` _worldlocation (+ _worldlocation (* _worlddirection 10000.0)) "TraceTypeQuery3"))
  (bind (_bblockinghit _binitialoverlap _time _distance _location) (`GameplayStatics.BreakHitResult` _outhit))
  (if _bblockinghit
    (bind _returnvalue (`GameplayStatics.GetActorOfClass` "/Game/SoundWall/SoundWallGrid/WallGridManager.WallGridManager_C"))
    (bind _outputvector (`/Game/SoundWall/SoundWallGrid/WallGridManager.GetClosestGridPosition` _returnvalue _location))
    (`self.K2_SetActorLocation` (`self.PlaceableActor`) _outputvector false false)))

(fn `UserConstructionScript`)